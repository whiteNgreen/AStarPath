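; BP_Node is a node actor whose mesh color shows its role in what appears to be a pathfinding visualization.
; It starts white on BeginPlay.
; The MatChange event switches on a Click state (none, start, target, path or checked) and sets the matching solid-color material.
; The node contains no search logic, and a leftover toggle of its Clicked flag is never run.
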(event EventBeginPlay
  (Rendering|Material|SetMaterial (Variables|Character|GetMesh) 0 "/Game/Materials/MI_White.MI_White"))

(event Collision|EventActorBeginOverlap
  (params (OtherActor :type Actor%20Object%20Reference)))

(event EventTick
  (params (DeltaSeconds :type Float%20%28single-precision%29)))

(event EventMatChange
  (params (click :type EMatType%20Enum :default "CL_None"))
  (switch Utilities|FlowControl|Switch|SwitchonEMatType click
    (:CL_None
      (Rendering|Material|SetMaterial (Variables|Character|GetMesh) 0 "/Game/Materials/MI_White.MI_White"))
    (:CL_Start
      (Rendering|Material|SetMaterial (Variables|Character|GetMesh) 0 "/Game/Materials/MI_Red.MI_Red"))
    (:CL_Target
      (Rendering|Material|SetMaterial (Variables|Character|GetMesh) 0 "/Game/Materials/MI_Blue.MI_Blue"))
    (:CL_Path
      (Rendering|Material|SetMaterial (Variables|Character|GetMesh) 0 "/Game/Materials/MI_Orange.MI_Orange"))
    (:CL_Checked
      (Rendering|Material|SetMaterial (Variables|Character|GetMesh) 0 "/Game/Materials/MI_Green.MI_Green"))))

(fn ConstructionScript)